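; Custom Game Instance that persists the player's settings across sessions through a BP_SettingsSave save game.
; On Init it loads the settings slot, creating a fresh save object if none is found, then applies the saved overall quality level through Game User Settings with VSync always enabled.
; On Shutdown it writes the settings back to the slot, with debug prints reporting load, apply and save results.
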(event `self.ReceiveInit`
  (`self.LoadSettings`)
  (`self.Apply Settings`))

(event `self.ReceiveShutdown`
  (`self.Save Settings`))

(fn `Apply Settings`
  (bind _settings (`self.Settings`))
  (bind _overallqualitylevel (`/Game/Game/BP_SettingsSave.OverallQualityLevel` _settings))
  (`/Engine/EditorBlueprintResources/StandardMacros.IsValid` _settings
    (:`Is Valid`
      (bind _returnvalue (`GameUserSettings.GetGameUserSettings`))
      (`/Engine/EditorBlueprintResources/StandardMacros.IsValid` _returnvalue
        (:`Is Valid`
          (`GameUserSettings.SetOverallScalabilityLevel` _returnvalue _overallqualitylevel)
          (`KismetSystemLibrary.PrintString` (`KismetStringLibrary.Conv_IntToString` _overallqualitylevel))
          (`GameUserSettings.SetVSyncEnabled` _returnvalue true)
          (`GameUserSettings.ApplySettings` _returnvalue true)
          (`KismetSystemLibrary.PrintString` "Settings Applied"))))))

(fn `LoadSettings`
  (bind _returnvalue (`GameplayStatics.LoadGameFromSlot` (`self.SettingsSlot`)))
  (bind _asbp_settings_save (cast `/Game/Game/BP_SettingsSave` _returnvalue)
    (:`then`
      (set `self.Settings` _asbp_settings_save)
      (`KismetSystemLibrary.PrintString` "Setting Loaded"))
    (:`CastFailed`
      (bind _returnvalue_2 (`GameplayStatics.CreateSaveGameObject` "/Game/Game/BP_SettingsSave.BP_SettingsSave_C"))
      (set `self.Settings` _returnvalue_2))))

(fn `Save Settings`
  (bind _returnvalue (`GameplayStatics.SaveGameToSlot` (`self.Settings`) (`self.SettingsSlot`)))
  (if _returnvalue
    (`KismetSystemLibrary.PrintString` "Settings Saved")
    (else
      (`KismetSystemLibrary.PrintString` "Failed To Save Game Settings"))))